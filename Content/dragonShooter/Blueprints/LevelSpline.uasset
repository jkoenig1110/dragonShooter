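; Level spline actor that carries the playfield along a path segment and fires SpawnTriggers along the way.
; On init it gathers triggers tagged with its own object name, links them to the playfield and sorts them by time.
; A timeline scaled by spline length and speed moves the playfield, then activates NextSpline when finished.
; Tick fires and removes triggers whose time the timeline has reached.
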(event Custom|InitLevelSpline
  (params (InPlayfield :type Playfield%20Object%20Reference))
  ;[1 1 1] Populate array of triggers
  (Variables|Default|SetPlayFieldRef InPlayfield)
  (bind _outactors (Actor|GetAllActorswithTag (Utilities|String|StringToName (Utilities|GetObjectName self))))
  (for _array_element _outactors
    (bind _asspawn_trigger (Utilities|Casting|CastToSpawnTrigger _array_element))
    (Utilities|Array|Add (Variables|Default|GetTriggerList) _asspawn_trigger)
    (Variables|/Game/dragonShooter/Blueprints/SpawnTrigger.SpawnTrigger_C|SetTriggerPlayfieldRef _asspawn_trigger (Variables|Default|GetPlayFieldRef)))
  (bind _sortedtriggers (CallFunction|SortTriggers (Variables|Default|GetTriggerList)))
  (Variables|Default|SetTriggerList _sortedtriggers))

(event Custom|ActivateLevelSpline
  (bind _spline (Variables|Default|GetSpline))
  (bind _nextspline (Variables|Default|GetNextSpline))
  (bind _playfieldref (Variables|Default|GetPlayFieldRef))
  ;[1 1 1] Set speed
  (Actor|Tick|SetActorTickEnabled true)
  (Components|Timeline|SetPlayRate (Variables|Default|GetPlayerLocTimeline) (/ 1.0 (/ (Spline|GetSplineLength (Variables|Default|GetSpline)) (Variables|Default|GetPlayfieldSpeed))))
  ;[1 1 1] Do movement
  (bind _splinetime (Timeline|PlayerLocTimeline PlayFromStart)
    (:Update
      (Transformation|SetActorLocation _playfieldref (Spline|GetLocationatTime _spline _splinetime "World" true) false false)
      (Transformation|SetActorRotation _playfieldref (Math|Rotator|MakeRotator (.roll (Class|SplineComponent|GetRotationatTime _spline _splinetime "World" true)) 0.0 (.yaw (Class|SplineComponent|GetRotationatTime _spline _splinetime "World" true))))
      (Development|PrintString (Utilities|String|ToString(Float) _splinetime) true true "(R=1.000000,G=0.000000,B=0.498242,A=1.000000)" 0.0))
    (:Finished
      (Utilities|IsValid _nextspline
        (:Is%20Valid
          (CallFunction|ActivateLevelSpline _nextspline))))))

(event EventBeginPlay)

(event Collision|EventActorBeginOverlap
  (params (OtherActor :type Actor%20Object%20Reference)))

(event EventTick
  (params (DeltaSeconds :type Float%20%28single-precision%29))
  (bind _triggerlist (Variables|Default|GetTriggerList))
  (Utilities|FlowControl|Sequence
    (:then_1
      (if (not (== (Utilities|Array|LastIndex _triggerlist) 0))
        ;[1 1 1] Spawn triggers with time > SplineTime, break if time < SplineTime
        (bind _array_element (Utilities|Array|ForEachLoopwithBreak _triggerlist :!label _label)
          (:LoopBody
            (if (>= (stale Custom|ActivateLevelSpline _splinetime) (Variables|/Game/dragonShooter/Blueprints/SpawnTrigger.SpawnTrigger_C|GetTime _array_element))
              (Default|Trigger _array_element)
              (Math|Integer|IncrementInt (Variables|Default|GetToRemove))
              (else
                (goto _label Break))))
          (:Completed
            ;[1 1 1] Remove trigger references that have been triggered
            (for _index (range 1 (Variables|Default|GetToRemove))
              (Utilities|Array|RemoveIndex _triggerlist (- _index 1)))
            (Variables|Default|SetToRemove 0)))))))

(fn ConstructionScript)

(fn SortTriggers
  (params (InActors :type Array%20of%20Spawn%20Trigger%20Object%20References))
  (bind _sortedlist (LocalVariables|GetSortedList))
  (Utilities|Array|Add (LocalVariables|GetSortedList) (Utilities|Array|Get(acopy) InActors))
  (for _index (range 1 (Utilities|Array|LastIndex InActors))
    (bind (_array_element _array_index) (Utilities|Array|ForEachLoopwithBreak _sortedlist :!label _label)
      (:LoopBody
        (if (>= (Variables|/Game/dragonShooter/Blueprints/SpawnTrigger.SpawnTrigger_C|GetTime _array_element) (Variables|/Game/dragonShooter/Blueprints/SpawnTrigger.SpawnTrigger_C|GetTime (Utilities|Array|Get(acopy) InActors _index)))
          (Utilities|Array|Insert _sortedlist (Utilities|Array|Get(acopy) InActors _index) _array_index)
          (goto _label Break)
          (elif (== _array_index (Utilities|Array|LastIndex _sortedlist))
            (Utilities|Array|Add _sortedlist (Utilities|Array|Get(acopy) InActors _index))
            (goto _label Break))))))
  (return (LocalVariables|GetSortedList)))