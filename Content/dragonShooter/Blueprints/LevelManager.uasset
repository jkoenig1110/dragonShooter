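; LevelManager is the per-level bootstrap actor for the dragon shooter, starting the playfield and spline-based level path.
; On BeginPlay it prints an error if more than one manager exists, then spawns a Playfield at the first point of StartSpline and initializes it.
; It then passes that Playfield to every LevelSpline's init and activates StartSpline to begin the level.
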(event EventBeginPlay
  (Utilities|FlowControl|Sequence
    (:then_0
      (bind _outactors (Actor|GetAllActorsOfClass "LevelManager_C"))
      (if (> (Utilities|Array|Length _outactors) 1)
        (Development|PrintString "ERROR: More than one level manager")))
    (:then_1
      (bind _returnvalue (Game|SpawnActorfromClass "/Game/dragonShooter/Blueprints/PlayField.Playfield_C" (Math|Conversions|ToTransform(Vector) (Spline|GetLocationatSplinePoint (Variables|/Game/dragonShooter/Blueprints/LevelSpline.LevelSpline_C|GetSpline (Variables|Default|GetStartSpline)) 0 "World")) "Undefined" 0 0))
      (bind _output_get (Variables|Default|SetPlayfieldRef _returnvalue))
      (Default|InitPlayfield _output_get))
    (:then_2
      (bind _outactors_2 (Actor|GetAllActorsOfClass "/Game/dragonShooter/Blueprints/LevelSpline.LevelSpline_C"))
      (for _array_element _outactors_2
        (Default|InitLevelSpline _array_element (Variables|Default|GetPlayfieldRef))))
    (:then_3
      (Default|ActivateLevelSpline (Variables|Default|GetStartSpline)))))

(event Collision|EventActorBeginOverlap
  (params (OtherActor :type Actor%20Object%20Reference)))

(event EventTick
  (params (DeltaSeconds :type Float%20%28single-precision%29)))

(fn ConstructionScript)