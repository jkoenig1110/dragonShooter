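; PlayField actor for the dragon shooter that hosts the player, camera and enemies inside a configurable box-bounded area.
; InitPlayfield spawns, possesses and attaches the DragonBP; Tick flags screen-edge blocking from its projected position.
; ViewChange cycles side, top and rear views, lerping camera and dragon on a timeline.
; SpawnEnemyAttached attaches enemies and copies a template spline into each; NearBox destroys enemies that overlap it.
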(event Custom|KillBoxOverlap
  (params (OverlappedComponent :type Primitive%20Component%20Object%20Reference) (OtherActor :type Actor%20Object%20Reference) (OtherComp :type Primitive%20Component%20Object%20Reference) (OtherBodyIndex :type Integer) (bFromSweep :type Boolean) (SweepResult :type Hit%20Result%20Structure%20%28by%20ref%29))
  (bind _asenemy_base (Utilities|Casting|CastToEnemy_Base OtherActor))
  (Actor|DestroyActor _asenemy_base))

(event Custom|ViewChange
  (bind _self self)
  (bind _dragonref (Variables|Default|GetDragonRef))
  (bind _dragonref_2 (Variables|Default|GetDragonRef))
  (bind _topview (Variables|Default|GetTopView))
  (bind _sideview (Variables|Default|GetSideView))
  (bind _rearview (Variables|Default|GetRearView))
  (bind _returnvalue (Transformation|GetActorForwardVector _self))
  (Variables|Default|SetRepositionStartLoc (Transformation|GetActorLocation _dragonref))
  (Variables|/Game/dragonShooter/Blueprints/DragonBP.DragonBP_C|SetInTransition _dragonref_2 true)
  (bind _newtrack_0 (Timeline|Transition PlayFromStart)
    (:Update
      (Transformation|SetWorldTransform (Variables|Default|GetCamera) (Math|Transform|Lerp(Transform) (Transformation|GetWorldTransform (Utilities|Select :Index (Variables|Default|GetCurrentPerspective) :NewEnumerator0 _sideview :NewEnumerator1 _topview :NewEnumerator2 _rearview)) (Transformation|GetWorldTransform (Utilities|Select :Index (Utilities|Enum|ByteToEnumEViewPersp (Class|KismetMathLibrary|PercentByteByte (+ (Variables|Default|GetCurrentPerspective) 1) 3)) :NewEnumerator0 _sideview :NewEnumerator1 _topview :NewEnumerator2 _rearview)) _newtrack_0) false false)
      (Transformation|SetActorLocation _dragonref (Math|Vector|Lerp(Vector) (Variables|Default|GetRepositionStartLoc) (+ (Utilities|Select :Index (Utilities|Enum|ByteToEnumEViewPersp (Class|KismetMathLibrary|PercentByteByte (+ (Variables|Default|GetCurrentPerspective) 1) 3)) :NewEnumerator0 (* _returnvalue -1.5e+03) :NewEnumerator1 (* _returnvalue -1e+03) :NewEnumerator2 (* _returnvalue -7.5e+02)) (Transformation|GetActorLocation _self)) _newtrack_0) false false))
    (:Finished
      (Variables|Default|SetCurrentPerspective (Utilities|Enum|ByteToEnumEViewPersp (Class|KismetMathLibrary|PercentByteByte (+ (Variables|Default|GetCurrentPerspective) 1) 3)))
      (Variables|/Game/dragonShooter/Blueprints/DragonBP.DragonBP_C|SetInTransition _dragonref_2 false))))

(event Custom|InitPlayfield
  (bind _returnvalue (Game|GetPlayerController 0))
  (bind _defaultsceneroot (Variables|Default|GetDefaultSceneRoot))
  (Utilities|FlowControl|Sequence
    (:then_0
      ;[1 1 1] Player Setup
      (bind _returnvalue_2 (Game|SpawnActorfromClass "/Game/dragonShooter/Blueprints/DragonBP.DragonBP_C" (Math|Transform|MakeTransform (+ (Transformation|GetWorldLocation _defaultsceneroot) (* (Math|Vector|GetForwardVector _defaultsceneroot) (+ (Variables|BoundsBoxes|GetNearBoxOffset) 2e+02))) "0, 0, 0" "1,1,1") "Undefined" 0 0))
      (Variables|Default|SetDragonRef _returnvalue_2)
      (Pawn|Possess _returnvalue (Variables|Default|GetDragonRef))
      (Pawn|Components|CharacterMovement|SetMovementMode (Variables|/Script/Engine.Character|GetCharacterMovement (Variables|Default|GetDragonRef)) "MOVE_Flying" 0)
      (Game|Player|SetViewTargetwithBlend _returnvalue self 0.0 "VTBlend_Linear" 0.0 false)
      (Transformation|AttachActorToActor (Variables|Default|GetDragonRef) self "None" "KeepWorld" "KeepWorld" "KeepWorld" true)
      (Variables|/Game/dragonShooter/Blueprints/DragonBP.DragonBP_C|SetIsAttached (Variables|Default|GetDragonRef) true)
      (Variables|/Game/dragonShooter/Blueprints/DragonBP.DragonBP_C|SetPlayFieldRef (Variables|Default|GetDragonRef) self)
      (Transformation|SetAbsolute (Variables|/Script/Engine.Character|GetCapsuleComponent (Variables|Default|GetDragonRef)) false true false)
      (Variables|/Game/dragonShooter/Blueprints/DragonShooter_Controller.DragonShooter_Controller_C|SetControllerDragonRef (.AsDragon%20Shooter%20Controller (Utilities|Casting|CastToDragonShooter_Controller (Game|GetPlayerController 0))) (Variables|Default|GetDragonRef)))
    (:then_1
      (Collision|AssignOnComponentBeginOverlap (Variables|Default|GetNearBox) (delegate Custom|KillBoxOverlap)))))

(event EventTick
  (params (DeltaSeconds :type Float%20%28single-precision%29))
  (bind _returnvalue (Game|GetPlayerController 0))
  (bind _returnvalue_2 (Viewport|GetViewportSize))
  (bind _dragonref (Variables|Default|GetDragonRef))
  (bind _returnvalue_3 (Transformation|GetActorLocation _dragonref))
  (bind _screenlocation (Class|PlayerController|ProjectWorldLocationtoScreen _returnvalue _returnvalue_3 false))
  (bind _returnvalue_4 (/ _screenlocation _returnvalue_2))
  (bind (_x _y) (Math|Vector2D|BreakVector2D _returnvalue_4))
  ;[1 1 1] Set Block Flags
  (Utilities|IsValid _dragonref
    (:Is%20Valid
      (Utilities|Struct|SetmembersinBlockFlags (Variables|/Game/dragonShooter/Blueprints/DragonBP.DragonBP_C|GetBlockLRUD _dragonref) (<= _x 0.05) (>= _x 0.95) (<= _y 0.05) (>= _y 0.95))
      (Transformation|SetActorRotation (Variables|Default|GetDragonRef) (Transformation|GetWorldRotation (Variables|Default|GetSphere))))))

(fn ConstructionScript
  (bind _nearbox (Variables|Default|GetNearBox))
  (bind _rightbox (Variables|Default|GetRightBox))
  (bind _sideboxesxoffset (Variables|BoundsBoxes|GetSideBoxesXOffset))
  (bind _sideboxeswidth (Variables|BoundsBoxes|GetSideBoxesWidth))
  (bind _leftbox (Variables|Default|GetLeftBox))
  (bind _sideboxesangle (Variables|BoundsBoxes|GetSideBoxesAngle))
  (bind _sideboxesyoffset (Variables|BoundsBoxes|GetSideBoxesYOffset))
  (bind _boxesheight (Variables|BoundsBoxes|GetBoxesHeight))
  (bind _farbox (Variables|Default|GetFarBox))
  (Transformation|AddRelativeLocation _nearbox (Math|Vector|MakeVector (Variables|BoundsBoxes|GetNearBoxOffset) 0.0 0.0) false false)
  (Components|Box|SetBoxExtent _nearbox (Math|Vector|MakeVector 1e+02 (Variables|BoundsBoxes|GetNearBoxWidth) _boxesheight) false)
  (Transformation|AddRelativeLocation _farbox (Math|Vector|MakeVector (Variables|BoundsBoxes|GetFarBoxOffset) 0.0 0.0) false false)
  (Components|Box|SetBoxExtent _farbox (Math|Vector|MakeVector 1e+02 (Variables|BoundsBoxes|GetFarBoxWidth) _boxesheight) false)
  (Transformation|AddRelativeLocation _rightbox (Math|Vector|MakeVector _sideboxesxoffset _sideboxesyoffset 0.0) false false)
  (Components|Box|SetBoxExtent _rightbox (Math|Vector|MakeVector 1e+02 _sideboxeswidth _boxesheight) false)
  (Transformation|AddRelativeRotation _rightbox (Math|Rotator|MakeRotator 0.0 0.0 _sideboxesangle) false false)
  (Transformation|AddRelativeLocation _leftbox (Math|Vector|MakeVector _sideboxesxoffset (* -1 _sideboxesyoffset) 0.0) false false)
  (Components|Box|SetBoxExtent _leftbox (Math|Vector|MakeVector 1e+02 _sideboxeswidth _boxesheight) false)
  (Transformation|AddRelativeRotation _leftbox (Math|Rotator|MakeRotator 0.0 0.0 (* -1 _sideboxesangle)) false false))

(fn SpawnEnemyAttached
  (params (Offset :type Vector) (EnemyClass :type Enemy%20Base%20Class%20Reference) (MovementSplineType :type EEnemySpline%20Enum :default "NewEnumerator0") (EnemySpeed :type Float%20%28single-precision%29))
  (bind _forwardsstraight (Variables|Default|GetForwardsStraight))
  (bind _bigwaves (Variables|Default|GetBigWaves))
  (bind _splinearray (LocalVariables|GetSplineArray))
  (bind _returnvalue (Utilities|Select :Index MovementSplineType :NewEnumerator0 _forwardsstraight :NewEnumerator1 _bigwaves))
  (bind _returnvalue_2 (Game|SpawnActorfromClass EnemyClass (Math|Transform|MakeTransform (+ (Transformation|GetWorldLocation (Variables|Default|GetSphere)) (* (Transformation|GetActorRightVector) (.y Offset))) (Math|Rotator|MakeRotfromXZ (* (Transformation|GetActorForwardVector) -1) (Transformation|GetActorUpVector)) "1,1,1") "Undefined" 0 2e+02 0))
  (Transformation|AttachActorToActor _returnvalue_2 self "None" "KeepWorld" "KeepWorld" "KeepWorld" true)
  (Spline|ClearSplinePoints (Variables|/Game/dragonShooter/Blueprints/Enemies/Enemy_Base.Enemy_Base_C|GetSpline _returnvalue_2) true)
  (for _index (range 0 (- (Spline|GetNumberOfSplinePoints _returnvalue) 1))
    (Utilities|Array|Add _splinearray (Utilities|Struct|MakeSplinePoint (Math|Conversions|ToFloat(Integer) _index) (Spline|GetLocationatSplinePoint _returnvalue _index "Local") (Spline|GetArriveTangentatSplinePoint _returnvalue _index "Local") (Spline|GetLeaveTangentatSplinePoint _returnvalue _index "Local") (Spline|GetRotationatSplinePoint _returnvalue _index "Local") (Spline|GetScaleatSplinePoint _returnvalue _index) (Class|SplineComponent|GetSplinePointType _returnvalue _index))))
  (for _array_element _splinearray
    (Class|SplineComponent|AddPoint (Variables|/Game/dragonShooter/Blueprints/Enemies/Enemy_Base.Enemy_Base_C|GetSpline _returnvalue_2) _array_element true))
  (Default|ActivateEnemy _returnvalue_2))