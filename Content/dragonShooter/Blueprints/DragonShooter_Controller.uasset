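; Player controller for the dragon shooter that steers the referenced dragon by mouse or by Up/Right input axes.
; BeginPlay creates crosshair and line widgets; when mouse control is enabled, Tick moves the crosshair to the cursor and stretches the line from the dragon to it.
; The cursor's screen offset from the projected dragon position, scaled and clamped per axis, drives MoveUp and MoveRight like an analog stick.
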(event EventBeginPlay
  (bind _returnvalue (UserInterface|CreateWidget "/Game/dragonShooter/UI/Crosshair.Crosshair_C" self))
  (UserInterface|Viewport|AddtoViewport _returnvalue 0)
  (bind _returnvalue_2 (UserInterface|CreateWidget "/Game/dragonShooter/UI/Line.Line_C"))
  (UserInterface|Viewport|AddtoViewport _returnvalue_2 0)
  (bind _returnvalue_3 (Class|WidgetLayoutLibrary|GetMousePositiononViewport))
  (Class|UserWidget|SetPositioninViewport _returnvalue _returnvalue_3 true))

(event EventTick
  (params (DeltaSeconds :type Float%20%28single-precision%29))
  (bind _self self)
  (bind _controllerdragonref (Variables|Default|GetControllerDragonRef))
  (bind _controllerdragonref_2 (Variables|Default|GetControllerDragonRef))
  (bind _returnvalue (Transformation|GetActorLocation _controllerdragonref))
  (if (Variables|Default|GetMouseControlEnabled)
    (bind _returnvalue_2 (Class|WidgetLayoutLibrary|GetPlayerScreenWidgetGeometry self))
    (bind _returnvalue_3 (Class|WidgetLayoutLibrary|GetMousePositiononViewport))
    (Class|UserWidget|SetPositioninViewport (stale EventBeginPlay _returnvalue) (.PixelPosition (Class|SlateBlueprintLibrary|LocaltoViewport _returnvalue_2 _returnvalue_3)) true)
    (Variables|/Game/dragonShooter/UI/Line.Line_C|SetStart (stale EventBeginPlay _returnvalue_2) (+ (.ViewportPosition (Class|SlateBlueprintLibrary|LocaltoViewport _returnvalue_2 (.ScreenPosition (Class|WidgetLayoutLibrary|ProjectWorldLocationtoWidgetPosition _self _returnvalue)))) "(X=0.000000,Y=-32.000000)"))
    (Variables|/Game/dragonShooter/UI/Line.Line_C|SetEnd (stale EventBeginPlay _returnvalue_2) (+ (.ViewportPosition (Class|SlateBlueprintLibrary|LocaltoViewport _returnvalue_2 _returnvalue_3)) "(X=16.000000,Y=16.000000)"))
    (Default|MoveUp _controllerdragonref_2 (* (.y (Class|KismetMathLibrary|ClampAxes2D (/ (- (.PixelPosition (Class|SlateBlueprintLibrary|LocaltoViewport _returnvalue_2 _returnvalue_3)) (.ScreenPosition (Class|GameplayStatics|ProjectWorldtoScreen _self _returnvalue false))) (Math|Vector2D|MakeVector2D 2e+02 2e+02)) -1.0 1.0)) -1.0))
    (Default|MoveRight _controllerdragonref_2 (.x (Class|KismetMathLibrary|ClampAxes2D (/ (- (.PixelPosition (Class|SlateBlueprintLibrary|LocaltoViewport _returnvalue_2 _returnvalue_3)) (.ScreenPosition (Class|GameplayStatics|ProjectWorldtoScreen _self _returnvalue false))) (Math|Vector2D|MakeVector2D 2e+02 2e+02)) -1.0 1.0)))))

(event Input|AxisEvents|InputAxisUp
  (params (AxisValue :type Float%20%28single-precision%29))
  (Default|MoveUp (Variables|Default|GetControllerDragonRef) AxisValue))

(event Input|AxisEvents|InputAxisRight
  (params (AxisValue :type Float%20%28single-precision%29))
  (Default|MoveRight (Variables|Default|GetControllerDragonRef) AxisValue))

(fn ConstructionScript)