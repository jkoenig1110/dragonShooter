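; BPGustBox is a wind gust volume that slows the player's dragon while it is inside.
; Its CollisionBox overlap events cast to DragonBP, halving the character movement's MaxFlySpeed on entry and doubling it on exit.
; An older gated approach that eased the speed change using WindSpeed and clamp limits remains as disconnected, obsolete nodes, alongside empty CloseGate events.
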(event OnComponentBeginOverlap(CollisionBox)
  (params (OverlappedComponent :type Primitive%20Component%20Object%20Reference) (OtherActor :type Actor%20Object%20Reference) (OtherComp :type Primitive%20Component%20Object%20Reference) (OtherBodyIndex :type Integer) (bFromSweep :type Boolean) (SweepResult :type Hit%20Result%20Structure%20%28by%20ref%29))
  (bind _asdragon_bp (Utilities|Casting|CastToDragonBP OtherActor))
  (Variables|/Script/Engine.CharacterMovementComponent|SetMaxFlySpeed (Variables|/Script/Engine.Character|GetCharacterMovement _asdragon_bp) (/ (Variables|/Script/Engine.CharacterMovementComponent|GetMaxFlySpeed (Variables|/Script/Engine.Character|GetCharacterMovement _asdragon_bp)) 2.0)))

(event OnComponentEndOverlap(CollisionBox)
  (params (OverlappedComponent :type Primitive%20Component%20Object%20Reference) (OtherActor :type Actor%20Object%20Reference) (OtherComp :type Primitive%20Component%20Object%20Reference) (OtherBodyIndex :type Integer))
  (bind _asdragon_bp (Utilities|Casting|CastToDragonBP OtherActor))
  (Variables|/Script/Engine.CharacterMovementComponent|SetMaxFlySpeed (Variables|/Script/Engine.Character|GetCharacterMovement _asdragon_bp) (* (Variables|/Script/Engine.CharacterMovementComponent|GetMaxFlySpeed (Variables|/Script/Engine.Character|GetCharacterMovement _asdragon_bp)) 2.0)))

(event Custom|Close%20Gate%201)

(event Custom|Close%20Gate%202)

(event EventBeginPlay)

(event EventTick
  (params (DeltaSeconds :type Float%20%28single-precision%29)))

(fn ConstructionScript)