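; Level-placed trigger that spawns enemies attached to the moving playfield at a point along a level spline.
; Construction script tags it with the spline's name, finds the nearest spline point and normalized time, and positions spawn point, enemy mesh and playfield previews.
; Trigger attaches it to the playfield, then spawns immediately or on a LoopInterval timer, passing speed and movement path, and destroys itself once NumToSpawn is reached.
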(event Custom|Trigger
  (bind _loopcount (Variables|Default|GetLoopCount))
  (bind _loopinterval (Variables|Default|GetLoopInterval))
  ;[1 1 1] Handle single spawn or multiple delayed
  (Transformation|AttachActorToActor (Variables|Default|GetTriggerPlayfieldRef) "None" "KeepWorld" "KeepWorld" "KeepWorld" true)
  (if (== _loopinterval 0.0)
    (if (< _loopcount (Variables|Default|GetNumToSpawn))
      (Math|Integer|IncrementInt _loopcount
        (:%20%20
          (Default|SpawnEnemyAttached (Variables|Default|GetTriggerPlayfieldRef) (Transformation|GetWorldLocation (Variables|Default|GetSpawnHere)) (Variables|Default|GetEnemyToSpawn) (Variables|Default|GetEnemySpeed) (Variables|Default|GetMovementSpline))
          (Development|PrintString (Utilities|String|Append "Spawn at " (Utilities|String|ToString(Float) (Variables|Default|GetTime))))
          (Utilities|Time|SetTimerbyEvent (delegate Custom|SpawnEnemy) _loopinterval :!label _label)))
      (else
        (Actor|DestroyActor)))
    (else
      (goto _label))))

(event Custom|SpawnEnemy
  (bind _loopcount (Variables|Default|GetLoopCount))
  (if (< _loopcount (Variables|Default|GetNumToSpawn))
    (Math|Integer|IncrementInt _loopcount
      (:%20%20
        (Default|SpawnEnemyAttached (Variables|Default|GetTriggerPlayfieldRef) (Transformation|GetWorldLocation (Variables|Default|GetSpawnHere)) (Variables|Default|GetEnemyToSpawn) (Variables|Default|GetEnemySpeed) (Variables|Default|GetMovementSpline))
        (Development|PrintString (Utilities|String|Append "Spawn at " (Utilities|String|ToString(Float) (Variables|Default|GetTime))))
        ;[1 1 1] Handle single spawn or multiple delayed
        (Utilities|Time|SetTimerbyEvent (delegate Custom|SpawnEnemy) (Variables|Default|GetLoopInterval))))
    (else
      (Actor|DestroyActor))))

(event EventBeginPlay
  ;[1 1 1] Warn if trigger does not have associated LevelSpline
  (if (not (Utilities|IsValid (Variables|Default|GetCheckSpline)))
    (Development|PrintString (Utilities|String|Append "ERROR " (Utilities|GetObjectName self) " CheckSpline reference not set!") true true "(R=1.000000,G=0.008681,B=0.000000,A=1.000000)" 4.0)))

(event Collision|EventActorBeginOverlap
  (params (OtherActor :type Actor%20Object%20Reference)))

(event EventTick
  (params (DeltaSeconds :type Float%20%28single-precision%29)))

(fn ConstructionScript
  (bind _returnvalue (Transformation|GetActorLocation))
  (bind _checkspline (Variables|Default|GetCheckSpline))
  (bind _spawnoffset (Variables|Default|GetSpawnOffset))
  (bind _checkspline_2 (Variables|Default|GetCheckSpline))
  (bind _enemytospawn (Variables|Default|GetEnemyToSpawn))
  (bind _spline (Variables|/Game/dragonShooter/Blueprints/LevelSpline.LevelSpline_C|GetSpline _checkspline))
  ;[1 1 1] Set data
  (Utilities|FlowControl|Sequence
    (:then_0
      (Utilities|Array|SetArrayElem (Variables|Actor|GetTags) 0 (Utilities|String|StringToName (Utilities|GetObjectName _checkspline)) true)
      (if (Utilities|IsValid _checkspline)
        (bind _output_get (Variables|Default|SetPointOnLevelSpline (Spline|FindLocationClosesttoWorldLocation _spline _returnvalue "World")))
        (Variables|Default|SetTime (CallFunction|FindTimeClosesttoLocation _returnvalue _spline))
        (Transformation|SetWorldLocation (Variables|Default|GetTriggerHere) _output_get false false)))
    (:then_1
      ;;[1 1 1] Set preview meshes
      (if (Utilities|ClassIsChildOf _enemytospawn "/Game/dragonShooter/Blueprints/Enemies/Enemy_SkeletalMesh.Enemy_SkeletalMesh_C")
        (Class|SkinnedMeshComponent|SetSkeletalMesh (Variables|Default|GetPreview_Skeletal) (Variables|/Script/Engine.SkinnedMeshComponent|GetSkeletalMesh (Class|GetClassObject|FindDefaultComponentbyClass _enemytospawn "/Script/Engine.SkeletalMeshComponent")) true)
        (else
          (Components|StaticMesh|SetStaticMesh (Variables|Default|GetPreview_Static) (Variables|/Script/Engine.StaticMeshComponent|GetStaticMesh (Class|GetClassObject|FindDefaultComponentbyClass _enemytospawn "/Script/Engine.StaticMeshComponent"))))))
    (:then_2
      (Transformation|SetWorldLocation (Variables|Default|GetSpawnHere) (+ (Variables|Default|GetPointOnLevelSpline) (+ (* (Transformation|GetActorForwardVector) (.x _spawnoffset)) (* (Transformation|GetActorUpVector) (.z _spawnoffset)) (* (Transformation|GetActorRightVector) (.y _spawnoffset)))) false false)
      (Rendering|SetVisibility (Variables|Default|GetPlayfieldPreview) (Variables|Default|GetShowPlayfield) false)
      (Transformation|SetWorldTransform (Variables|Default|GetPlayfieldPreview) (Math|Transform|MakeTransform (+ (Spline|GetLocationatTime (Variables|/Game/dragonShooter/Blueprints/LevelSpline.LevelSpline_C|GetSpline _checkspline_2) (Variables|Default|GetTime) "World" true) (Math|Vector|RotateVector (Math|Vector|MakeVector 3.6e+03 0.0 0.0) (Math|Rotator|MakeRotator (.Roll (Math|Rotator|BreakRotator (Class|SplineComponent|GetRotationatTime (Variables|/Game/dragonShooter/Blueprints/LevelSpline.LevelSpline_C|GetSpline _checkspline_2) (Variables|Default|GetTime) "World" true))) 0.0 (.Yaw (Math|Rotator|BreakRotator (Class|SplineComponent|GetRotationatTime (Variables|/Game/dragonShooter/Blueprints/LevelSpline.LevelSpline_C|GetSpline _checkspline_2) (Variables|Default|GetTime) "World" true)))))) (Math|Rotator|MakeRotator (.Roll (Math|Rotator|BreakRotator (Class|SplineComponent|GetRotationatTime (Variables|/Game/dragonShooter/Blueprints/LevelSpline.LevelSpline_C|GetSpline _checkspline_2) (Variables|Default|GetTime) "World" true))) 0.0 (.Yaw (Math|Rotator|BreakRotator (Class|SplineComponent|GetRotationatTime (Variables|/Game/dragonShooter/Blueprints/LevelSpline.LevelSpline_C|GetSpline _checkspline_2) (Variables|Default|GetTime) "World" true)))) "1,1,1") false false))))

(fn FindTimeClosesttoLocation
  (params (Location :type Vector) (Spline :type Spline%20Component%20Object%20Reference))
  (bind _returnvalue (Class|SplineComponent|FindInputKeyClosesttoWorldLocation Spline Location))
  (bind _returnvalue_2 (Math|Float|Truncate _returnvalue))
  (bind _returnvalue_3 (Spline|GetDistanceAlongSplineatSplinePoint Spline _returnvalue_2))
  (return (/ (+ _returnvalue_3 (* (- (Spline|GetDistanceAlongSplineatSplinePoint Spline (+ _returnvalue_2 1)) _returnvalue_3) (Math|Float|Fraction _returnvalue))) (Spline|GetDistanceAlongSplineatSplinePoint Spline (- (Spline|GetNumberOfSplinePoints Spline) 1)))))