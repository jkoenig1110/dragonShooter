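; Player dragon character for a shooter whose play field switches between side, top and rear views.
; Input moves it along the PlayField camera's axes, limited by per-direction block flags.
; Tick stops it at screen edges, uses traces to detach it from the PlayField near static geometry and reattach when clear, and eases it onto the current view plane outside transitions.
; Debug leftovers include Q view switching and radial damage tests.
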(event Custom|CustomEvent_0
  (params (DamagedActor :type Actor%20Object%20Reference) (Damage :type Float%20%28single-precision%29) (DamageType :type Damage%20Type%20Object%20Reference) (Origin :type Vector) (HitInfo :type Hit%20Result%20Structure) (InstigatedBy :type Controller%20Object%20Reference) (DamageCauser :type Actor%20Object%20Reference))
  (Development|PrintString "ouchie"))

(event Collision|EventActorBeginOverlap
  (params (OtherActor :type Actor%20Object%20Reference)))

(event EventTick
  (params (DeltaSeconds :type Float%20%28single-precision%29))
  (bind _returnvalue (Transformation|GetActorForwardVector))
  (bind _returnvalue_2 (Transformation|GetActorLocation))
  (bind _returnvalue_3 (Transformation|GetActorRotation))
  (bind _returnvalue_4 (Transformation|GetActorForwardVector))
  (bind _returnvalue_5 (Transformation|GetActorLocation))
  (bind _returnvalue_6 (Transformation|GetActorLocation))
  (bind _array (Utilities|Array|MakeArray "ObjectTypeQuery1"))
  (bind _playfieldref (Variables|Default|GetPlayFieldRef))
  (bind _capsulecomponent (Variables|Collision|GetCapsuleComponent))
  (bind _charactermovement (Variables|Character|GetCharacterMovement))
  (bind _returnvalue_7 (Components|Capsule|GetScaledCapsuleRadius _capsulecomponent))
  (bind _returnvalue_8 (Transformation|GetActorLocation _playfieldref))
  (bind _returnvalue_9 (Transformation|GetWorldLocation _capsulecomponent))
  (bind _returnvalue_10 (- _returnvalue_8 _returnvalue_2))
  (bind _returnvalue_11 (+ _returnvalue_7 1e+01))
  (bind _returnvalue_12 (Math|Vector|UnrotateVector _returnvalue_10 _returnvalue_3))
  (bind (_x _y _z) (Math|Vector|BreakVector _returnvalue_12))
  (Utilities|FlowControl|Sequence
    (:then_0
      ;[1 1 1] Negate Velocity at Edge of Screen
      (if (not (.ReturnValue (Class|PlayerController|ProjectWorldLocationtoScreen (Game|GetPlayerController 0) (+ (* (Variables|/Script/Engine.MovementComponent|GetVelocity _charactermovement) DeltaSeconds) (Transformation|GetActorLocation)) false)))
        (Variables|/Script/Engine.MovementComponent|SetVelocity _charactermovement "0, 0, 0")))
    (:then_1
      ;[1 1 1] Trace for Collisions and Attach/Detach
      (bind _returnvalue_13 (Collision|SphereTraceForObjects _returnvalue_9 (+ _returnvalue_9 (* (Transformation|GetActorUpVector) 1.0)) _returnvalue_11 _array false 0 "None"))
      (if _returnvalue_13
        (bind _index (Utilities|FlowControl|ForLoopwithBreak 0 8 :!label _label)
          (:LoopBody
            (bind _returnvalue_14 (Collision|LineTraceForObjects _returnvalue_6 (+ (Math|Vector|RotateVectorAroundAxis (Math|Vector|RotateVector (* _returnvalue _returnvalue_11) (Math|Rotator|MakeRotator 0.0 (* (Math|Conversions|ToFloat(Boolean) (Math|Conversions|ToBoolean(Integer) _index)) 45.0) 0.0)) (* _index 45.0) _returnvalue) _returnvalue_6) _array false 0 "None" true "(R=1.000000,G=0.000000,B=0.000000,A=1.000000)" "(R=0.000000,G=1.000000,B=0.000000,A=1.000000)" 1.0))
            (if _returnvalue_14
              (goto _label Break)))
          (:Completed
            (if _returnvalue_14
              (if (Variables|Default|GetIsAttached) ; Hit
                (Transformation|DetachFromActor "KeepWorld" "KeepWorld" "KeepWorld")
                (Variables|Default|SetIsAttached false))
              (else
                (if (not (Variables|Default|GetIsAttached)) :!label _label_2 ; No Hits
                  (Transformation|AttachActorToActor (Variables|Default|GetPlayFieldRef) "None" "KeepWorld" "KeepWorld" "KeepWorld" true)
                  (Variables|Default|SetIsAttached true))))))
        (else
          (goto _label_2))))
    (:then_2
      ;[1 1 1] Zero Location to View Plane
      (if (not (Variables|Default|GetInTransition))
        (Transformation|SetActorLocation (Math|Interpolation|VInterpTo _returnvalue_5 (+ (Utilities|Select :Index (Variables|/Game/dragonShooter/Blueprints/PlayField.Playfield_C|GetCurrentPerspective _playfieldref) :NewEnumerator0 (* (Transformation|GetActorRightVector) _y) :NewEnumerator1 (* (Transformation|GetActorUpVector) _z) :NewEnumerator2 (- (* _returnvalue_4 _x) (* _returnvalue_4 750))) _returnvalue_5) DeltaSeconds 1.0) true false)))))

(event EventBeginPlay
  (Game|Damage|ApplyRadialDamage 1.0 (Transformation|GetActorLocation) 1e+02 0 0 (Variables|Default|GetPlayFieldRef) 0 false "ECC_Visibility"))

(event Game|Damage|EventRadialDamage
  (params (DamageReceived :type Float%20%28single-precision%29) (DamageType :type Damage%20Type%20Object%20Reference) (Origin :type Vector :default "0, 0, 0") (HitInfo :type Hit%20Result%20Structure%20%28by%20ref%29) (InstigatedBy :type Controller%20Object%20Reference) (DamageCauser :type Actor%20Object%20Reference))
  (Development|PrintString "ouchie"))

(event Input|AxisEvents|InputAxisRight
  (params (AxisValue :type Float%20%28single-precision%29))
  (bind _blocklrud (Variables|Default|GetBlockLRUD))
  ;[1 1 1] Player Input
  (Class|PawnMovementComponent|AddInputVector (Variables|Character|GetCharacterMovement) (* (Math|Vector|GetRightVector (Variables|/Game/dragonShooter/Blueprints/PlayField.Playfield_C|GetCamera (Variables|Default|GetPlayFieldRef))) (Math|Float|Clamp(Float) AxisValue (* (Math|Conversions|ToInteger(Boolean) (not (.blockl _blocklrud))) -1.0) (* (Math|Conversions|ToInteger(Boolean) (not (.blockr _blocklrud))) 1.0))) false))

(event Input|AxisEvents|InputAxisUp
  (params (AxisValue :type Float%20%28single-precision%29))
  (bind _blocklrud (Variables|Default|GetBlockLRUD))
  ;[1 1 1] Player Input
  (Class|PawnMovementComponent|AddInputVector (Variables|Character|GetCharacterMovement) (* (Math|Vector|GetUpVector (Variables|/Game/dragonShooter/Blueprints/PlayField.Playfield_C|GetCamera (Variables|Default|GetPlayFieldRef))) (Math|Float|Clamp(Float) AxisValue (* (Math|Conversions|ToInteger(Boolean) (not (.blockd _blocklrud))) -1.0) (* (Math|Conversions|ToInteger(Boolean) (not (.blocku _blocklrud))) 1.0))) false))

(event Input|KeyboardEvents|Q
  (params (Key :type Key%20Structure :default "None"))
  ;[1 1 1] DEBUG: View Change
  (:Pressed
    (Default|ViewChange (Variables|Default|GetPlayFieldRef))))

(fn ConstructionScript)