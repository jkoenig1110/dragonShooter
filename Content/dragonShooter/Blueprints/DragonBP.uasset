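; Player dragon character for a shooter with side, top and rear views, moving relative to the PlayField actor.
; Mouse input opens gates that Tick pumps: a charged fireball released on button-up, auto-repeating ice shard spread, lightning orb and arcane blast, plus a montage-timed flame breath dealing radial damage.
; Tick also stops movement at screen edges, attaches or detaches from the PlayField using collision traces, and eases the dragon onto the view plane.
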(event Custom|IceShardAuto
  ;[1 0.3105 0.3603] Primary Abilities
  ;;[1 1 1] Ice Shard
  (Utilities|FlowControl|Gate true
    (:Exit
      (Utilities|FlowControl|DoOnce false
        (:Completed
          (Animation|PlayAnimMontage "/Game/QuadrapedCreatures/MountainDragon/Animations/Attack.Attack" 1.0 "None")
          (bind _returnvalue (Game|SpawnActorfromClass "/Game/dragonShooter/Projectiles/IceShard.IceShard_C" (Utilities|Aim (Variables|Character|GetMesh) (Variables|Default|GetAttackSocket) "1.000000,1.000000,1.000000") "Undefined" 0 4.0 false 0))
          (bind _returnvalue_2 (Game|SpawnActorfromClass "/Game/dragonShooter/Projectiles/IceShard.IceShard_C" (Utilities|AimLeft (Variables|Character|GetMesh) (Variables|Default|GetAttackSocket)) "Undefined" 0 4.0 false 0))
          (bind _returnvalue_3 (Game|SpawnActorfromClass "/Game/dragonShooter/Projectiles/IceShard.IceShard_C" (Utilities|AimRight (Variables|Character|GetMesh) (Variables|Default|GetAttackSocket)) "Undefined" 0 4.0 false 0))
          (Transformation|AttachActorToActor _returnvalue (Variables|Default|GetPlayFieldRef) "None" "KeepWorld" "KeepWorld" "KeepWorld" true)
          (Utilities|FlowControl|Delay 0.5)
          (CallFunction|ResetIceShard))))))

(event Custom|ResetIceShard
  ;[1 0.3105 0.3603] Primary Abilities
  ;;[1 1 1] Ice Shard
  (Utilities|FlowControl|DoOnce false) ; enters at Reset
)

(event Custom|Autofireball
  (bind _delta (Variables|Default|GetDelta))
  ;[1 0.3105 0.3603] Primary Abilities
  ;;[1 1 1] Fireball
  (Utilities|FlowControl|Gate true
    (:Exit
      (Variables|Default|SetFireball%20Damage (Math|Float|Clamp(Float) (Math|Interpolation|FInterptoConstant (Variables|Default|GetFireball%20Damage) 2e+01 _delta 12.0) 1.0 2e+01))
      (bind _output_get (Variables|Default|SetFireball%20Size (Math|Interpolation|VInterptoConstant (Variables|Default|GetFireball%20Size) "5.000000,5.000000,5.000000" _delta 5.0)))
      (Transformation|SetWorldScale3D (Variables|Default|GetFireCharge) _output_get))))

(event Custom|ResetFireball
  ;[1 0.3105 0.3603] Primary Abilities
  ;;[1 1 1] Fireball
  (Variables|Default|SetFireballSet false)
  (Utilities|FlowControl|DoOnce false) ; enters at Reset
)

(event Custom|Fireball
  (bind _delta (Variables|Default|GetDelta))
  ;[1 0.3105 0.3603] Primary Abilities
  ;;[1 1 1] Fireball
  (if (not (Variables|Default|GetIsFlameBreathActive))
    (Utilities|FlowControl|Gate true) ; enters at Open
  ))

(event Custom|CloseFireball
  ;[1 0.3105 0.3603] Primary Abilities
  ;;[1 1 1] Fireball
  (CallFunction|ShootFire)
  (Variables|Default|SetFireball%20Damage 1.0)
  (bind _output_get (Variables|Default|SetFireball%20Size "1.000000,1.000000,1.000000"))
  (Transformation|SetWorldScale3D (Variables|Default|GetFireCharge) _output_get)
  (CallFunction|FireFinish)
  (Components|Activation|Deactivate (Variables|Default|GetFireCharge)))

(event Custom|LightningOrbAuto
  ;[1 0.3105 0.3603] Primary Abilities
  ;;[1 1 1] Lightning Orb
  (Utilities|FlowControl|Gate true
    (:Exit
      (Utilities|FlowControl|DoOnce false
        (:Completed
          (Animation|PlayAnimMontage "/Game/QuadrapedCreatures/MountainDragon/Animations/Attack.Attack" 1.0 "None")
          (bind _returnvalue (Game|SpawnActorfromClass "/Game/dragonShooter/Projectiles/LightningBall.LightningBall_C" (Utilities|Aim (Variables|Character|GetMesh) (Variables|Default|GetAttackSocket) "1.000000,1.000000,1.000000") "Undefined" 0 1.0 0))
          (Transformation|AttachActorToActor _returnvalue (Variables|Default|GetPlayFieldRef) "None" "KeepWorld" "KeepWorld" "KeepWorld" true)
          (Utilities|FlowControl|Delay 0.1)
          (CallFunction|ResetOrb))))))

(event Custom|ResetOrb
  ;[1 0.3105 0.3603] Primary Abilities
  ;;[1 1 1] Lightning Orb
  (Utilities|FlowControl|DoOnce false) ; enters at Reset
)

(event Custom|Lightning%20Orb
  ;[1 0.3105 0.3603] Primary Abilities
  ;;[1 1 1] Lightning Orb
  (if (not (Variables|Default|GetIsFlameBreathActive))
    (Utilities|FlowControl|Gate true) ; enters at Open
  ))

(event Custom|CloseLightningOrb
  ;[1 0.3105 0.3603] Primary Abilities
  ;;[1 1 1] Lightning Orb
  (Utilities|FlowControl|Gate true) ; enters at Close
)

(event Custom|FlameBreathTick
  (bind _sphere (Variables|Default|GetSphere))
  ;[0.3837 0.3884 1] Alt Abilities
  ;;[1 1 1] Flame Breath
  (Utilities|FlowControl|Gate true
    (:Exit
      (bind _outactors (Actor|GetAllActorsOfClass "/Game/dragonShooter/Blueprints/Enemies/Enemy_Base.Enemy_Base_C"))
      (for _array_element _outactors
        (Utilities|IsValid _array_element
          (:Is%20Valid
            (Utilities|FlowControl|Delay 0.1)
            (Game|Damage|ApplyRadialDamage 1.0 (Transformation|GetWorldLocation _sphere) (Components|Sphere|GetScaledSphereRadius _sphere) "/Game/dragonShooter/Blueprints/DamageTypeRadial.DamageTypeRadial_C" 0 self 0 true "ECC_Visibility")))))))

(event Custom|CloseFlameBreathGate
  (bind _sphere (Variables|Default|GetSphere))
  ;[0.3837 0.3884 1] Alt Abilities
  ;;[1 1 1] Flame Breath
  (Utilities|FlowControl|Gate true) ; enters at Close
)

(event Custom|ResetFlameBreath
  (bind _torchfire_bp (Variables|Default|GetTorchfire_BP))
  ;[0.3837 0.3884 1] Alt Abilities
  ;;[1 1 1] Flame Breath
  (Utilities|FlowControl|DoOnce false) ; enters at Reset
)

(event Custom|SwitchPress
  ;[1 1 1] Main Attack Selector
  (if (Variables|Default|GetMousePressed)
    (CallFunction|CloseGate)
    (switch Utilities|FlowControl|Switch|SwitchonEPowerSelect (Variables|Default|GetPowerSelect)
      (:NewEnumerator0
        (CallFunction|Fireball)
        (Variables|Default|SetFireballSet true)
        (Components|Activation|Activate (Variables|Default|GetFireCharge) false))
      (:NewEnumerator1
        (CallFunction|IceShard))
      (:NewEnumerator2
        (CallFunction|LightningOrb))
      (:NewEnumerator3
        (CallFunction|ArcaneBlade)))))

(event Custom|ShootFire
  ;[1 0.3105 0.3603] Primary Abilities
  ;;[1 1 1] Fireball
  (Utilities|FlowControl|DoOnce false
    (:Completed
      (Animation|PlayAnimMontage "/Game/QuadrapedCreatures/MountainDragon/Animations/Attack.Attack" 1.0 "None")
      (bind _returnvalue (Game|SpawnActorfromClass "/Game/dragonShooter/Projectiles/Fireball.Fireball_C" (Utilities|Aim (Variables|Character|GetMesh) (Variables|Default|GetAttackSocket) (Variables|Default|GetFireball%20Size)) "Undefined" 0 (Variables|Default|GetFireball%20Damage) 0))
      (Variables|/Game/dragonShooter/Projectiles/Fireball.Fireball_C|SetExplosionSize _returnvalue (Variables|Default|GetFireball%20Size))
      (Transformation|AttachActorToActor _returnvalue (Variables|Default|GetPlayFieldRef) "None" "KeepWorld" "KeepWorld" "KeepWorld" true)
      (CallFunction|ResetFireball))))

(event Custom|FireFinish
  (bind _delta (Variables|Default|GetDelta))
  ;[1 0.3105 0.3603] Primary Abilities
  ;;[1 1 1] Fireball
  (Utilities|FlowControl|Gate true) ; enters at Close
)

(event Custom|Ice%20Shard
  ;[1 0.3105 0.3603] Primary Abilities
  ;;[1 1 1] Ice Shard
  (if (not (Variables|Default|GetIsFlameBreathActive))
    (Utilities|FlowControl|Gate true) ; enters at Open
  ))

(event Custom|CloseIceShard
  ;[1 0.3105 0.3603] Primary Abilities
  ;;[1 1 1] Ice Shard
  (Utilities|FlowControl|Gate true) ; enters at Close
)

(event Custom|Move%20Up
  (params (AxisValue :type Float%20%28single-precision%29))
  (bind _blocklrud (Variables|Default|GetBlockLRUD))
  ;[1 1 1] Movement
  (Class|PawnMovementComponent|AddInputVector (Variables|Character|GetCharacterMovement) (* (Math|Vector|GetUpVector (Variables|/Game/dragonShooter/Blueprints/PlayField.Playfield_C|GetTopView (Variables|Default|GetPlayFieldRef))) (Math|Float|Clamp(Float) AxisValue (* (Math|Conversions|ToInteger(Boolean) (not (.blockd _blocklrud))) -1.0) (* (Math|Conversions|ToInteger(Boolean) (not (.blocku _blocklrud))) 1.0))) false))

(event Custom|Move%20Right
  (params (AxisValue :type Float%20%28single-precision%29))
  (bind _blocklrud (Variables|Default|GetBlockLRUD))
  ;[1 1 1] Movement
  (Class|PawnMovementComponent|AddInputVector (Variables|Character|GetCharacterMovement) (* (Math|Vector|GetRightVector (Variables|/Game/dragonShooter/Blueprints/PlayField.Playfield_C|GetTopView (Variables|Default|GetPlayFieldRef))) (Math|Float|Clamp(Float) AxisValue (* (Math|Conversions|ToInteger(Boolean) (not (.blockl _blocklrud))) -1.0) (* (Math|Conversions|ToInteger(Boolean) (not (.blockr _blocklrud))) 1.0))) false)
  (CallFunction|LeftRightTilt AxisValue))

(event Custom|Flame%20Breath
  (bind _torchfire_bp (Variables|Default|GetTorchfire_BP))
  (bind _sphere (Variables|Default|GetSphere))
  ;[0.3837 0.3884 1] Alt Abilities
  ;;[1 1 1] Flame Breath
  (Utilities|FlowControl|Sequence
    (:then_0
      (Utilities|FlowControl|Gate true) ; enters at Open
    )
    (:then_1
      (Variables|Default|SetIsFlameBreathActive true)
      (Utilities|FlowControl|DoOnce false
        (:Completed
          (bind _returnvalue (Animation|PlayAnimMontage "/Game/QuadrapedCreatures/MountainDragon/Animations/ANIM_MOUNTAIN_DRAGON_FlyStationarySpreadFire_Montage.ANIM_MOUNTAIN_DRAGON_FlyStationarySpreadFire_Montage" 1.0 "None"))
          (Variables|Default|SetFlameDelay _returnvalue)
          (Components|Activation|Activate _torchfire_bp false)
          (Utilities|FlowControl|Delay (Variables|Default|GetFlameDelay))
          (CallFunction|CloseFlameBreathGate)
          (Components|Activation|Deactivate _torchfire_bp)
          (Variables|Default|SetIsFlameBreathActive false)
          (CallFunction|ResetFlameBreath))))))

(event Custom|Arcane%20Blade%20Auto
  ;[1 0.3105 0.3603] Primary Abilities
  ;;[1 1 1] Arcane Blade
  (Utilities|FlowControl|Gate true
    (:Exit
      (Utilities|FlowControl|DoOnce false
        (:Completed
          (Animation|PlayAnimMontage "/Game/QuadrapedCreatures/MountainDragon/Animations/Attack.Attack" 1.0 "None")
          (bind _returnvalue (Game|SpawnActorfromClass "/Game/dragonShooter/Projectiles/ArcaneBlast.ArcaneBlast_C" (Utilities|Aim (Variables|Character|GetMesh) (Variables|Default|GetAttackSocket) "1.000000,1.000000,1.000000") "Undefined" 0 1.0 0))
          (Transformation|AttachActorToActor _returnvalue (Variables|Default|GetPlayFieldRef) "None" "KeepWorld" "KeepWorld" "KeepWorld" true)
          (Utilities|FlowControl|Delay 1.0)
          (CallFunction|ResetArcaneBlade))))))

(event Custom|Reset%20Arcane%20Blade
  ;[1 0.3105 0.3603] Primary Abilities
  ;;[1 1 1] Arcane Blade
  (Utilities|FlowControl|DoOnce false) ; enters at Reset
)

(event Custom|Arcane%20Blade
  ;[1 0.3105 0.3603] Primary Abilities
  ;;[1 1 1] Arcane Blade
  (if (not (Variables|Default|GetIsFlameBreathActive))
    (Utilities|FlowControl|Gate true) ; enters at Open
  ))

(event Custom|Close%20Arcane%20Blade
  ;[1 0.3105 0.3603] Primary Abilities
  ;;[1 1 1] Arcane Blade
  (Utilities|FlowControl|Gate true) ; enters at Close
)

(event EventBeginPlay)

(event EventTick
  (params (DeltaSeconds :type Float%20%28single-precision%29))
  (bind _returnvalue (Transformation|GetActorForwardVector))
  (bind _returnvalue_2 (Transformation|GetActorLocation))
  (bind _returnvalue_3 (Transformation|GetActorRotation))
  (bind _returnvalue_4 (Transformation|GetActorForwardVector))
  (bind _returnvalue_5 (Transformation|GetActorLocation))
  (bind _returnvalue_6 (Transformation|GetActorLocation))
  (bind _array (Utilities|Array|MakeArray "ObjectTypeQuery1"))
  (bind _playfieldref (Variables|Default|GetPlayFieldRef))
  (bind _capsulecomponent (Variables|Collision|GetCapsuleComponent))
  (bind _charactermovement (Variables|Character|GetCharacterMovement))
  (bind _returnvalue_7 (Components|Capsule|GetScaledCapsuleRadius _capsulecomponent))
  (bind _returnvalue_8 (Transformation|GetActorLocation _playfieldref))
  (bind _returnvalue_9 (Transformation|GetWorldLocation _capsulecomponent))
  (bind _returnvalue_10 (- _returnvalue_8 _returnvalue_2))
  (bind _returnvalue_11 (+ _returnvalue_7 1e+01))
  (bind _returnvalue_12 (Math|Vector|UnrotateVector _returnvalue_10 _returnvalue_3))
  (bind (_x _y _z) (Math|Vector|BreakVector _returnvalue_12))
  (Variables|Default|SetDelta DeltaSeconds)
  (Utilities|FlowControl|Sequence
    (:then_0
      ;[1 1 1] Negate Velocity at Edge of Screen
      (if (not (.ReturnValue (Class|PlayerController|ProjectWorldLocationtoScreen (Game|GetPlayerController 0) (+ (* (Variables|/Script/Engine.MovementComponent|GetVelocity _charactermovement) DeltaSeconds) (Transformation|GetActorLocation)) false)))
        (Variables|/Script/Engine.MovementComponent|SetVelocity _charactermovement "0, 0, 0")))
    (:then_1
      ;[1 1 1] Trace for Collisions and Attach/Detach
      (bind _returnvalue_13 (Collision|SphereTraceForObjects _returnvalue_9 (+ _returnvalue_9 (* (Transformation|GetActorUpVector) 1.0)) _returnvalue_11 _array false 0 "None"))
      (if _returnvalue_13
        (bind _index (Utilities|FlowControl|ForLoopwithBreak 0 8 :!label _label)
          (:LoopBody
            (bind _returnvalue_14 (Collision|LineTraceForObjects _returnvalue_6 (+ (Math|Vector|RotateVectorAroundAxis (Math|Vector|RotateVector (* _returnvalue _returnvalue_11) (Math|Rotator|MakeRotator 0.0 (* (Math|Conversions|ToFloat(Boolean) (Math|Conversions|ToBoolean(Integer) _index)) 45.0) 0.0)) (* _index 45.0) _returnvalue) _returnvalue_6) _array false 0 "None" true "(R=1.000000,G=0.000000,B=0.000000,A=1.000000)" "(R=0.000000,G=1.000000,B=0.000000,A=1.000000)" 1.0))
            (if _returnvalue_14
              (goto _label Break)))
          (:Completed
            (if _returnvalue_14
              (if (Variables|Default|GetIsAttached) ; Hit
                (Transformation|DetachFromActor "KeepWorld" "KeepWorld" "KeepWorld")
                (Variables|Default|SetIsAttached false))
              (else
                (if (not (Variables|Default|GetIsAttached)) :!label _label_2 ; No Hits
                  (Transformation|AttachActorToActor (Variables|Default|GetPlayFieldRef) "None" "KeepWorld" "KeepWorld" "KeepWorld" true)
                  (Variables|Default|SetIsAttached true))))))
        (else
          (goto _label_2))))
    (:then_2
      ;[1 1 1] Zero Location to View Plane
      (if (not (Variables|Default|GetInTransition))
        (Transformation|SetActorLocation (Math|Interpolation|VInterpTo _returnvalue_5 (+ (Utilities|Select :Index (Variables|/Game/dragonShooter/Blueprints/PlayField.Playfield_C|GetCurrentPerspective _playfieldref) :NewEnumerator0 (* (Transformation|GetActorRightVector) _y) :NewEnumerator1 (* (Transformation|GetActorUpVector) _z) :NewEnumerator2 (- (* _returnvalue_4 _x) (* _returnvalue_4 750))) _returnvalue_5) DeltaSeconds 1.0) true false)))
    (:then_3
      ;[1 1 1] Reset tilt distance
      (Variables|Default|SetBanking (Math|Interpolation|FInterptoConstant (Variables|Default|GetBanking) 0.0 (Variables|Default|GetDelta) 1.5e+02)))
    (:then_4
      (CallFunction|AutofireFunct))))

(event Input|KeyboardEvents|Q
  (params (Key :type Key%20Structure :default "None")))

(event Input|MouseEvents|LeftMouseButton
  (params (Key :type Key%20Structure :default "None"))
  ;[1 1 1] Main Attack Selector
  (:Pressed
    (Variables|Default|SetMousePressed true)
    (switch Utilities|FlowControl|Switch|SwitchonEPowerSelect (Variables|Default|GetPowerSelect)
      (:NewEnumerator0
        (CallFunction|Fireball)
        (Variables|Default|SetFireballSet true)
        (Components|Activation|Activate (Variables|Default|GetFireCharge) false))
      (:NewEnumerator1
        (CallFunction|IceShard))
      (:NewEnumerator2
        (CallFunction|LightningOrb))
      (:NewEnumerator3
        (CallFunction|ArcaneBlade))))
  (:Released
    (Variables|Default|SetMousePressed false)
    (CallFunction|CloseGate)
    (if (Variables|Default|GetFireballSet)
      (CallFunction|CloseFireball))))

(event Input|MouseEvents|RightMouseButton
  (params (Key :type Key%20Structure :default "None"))
  ;[1 1 1] Alt Attack Selector
  (:Pressed
    (if (not (Variables|Default|GetMousePressed))
      (switch Utilities|FlowControl|Switch|SwitchonEAltPowerSelect (Variables|Default|GetAltPowerSelect)
        (:NewEnumerator0
          (CallFunction|FlameBreath)))))
  (:Released
    (CallFunction|CloseGateAlt)))

(event Input|KeyboardEvents|1
  (params (Key :type Key%20Structure :default "None"))
  ;[1 1 1] Attack Changer for Testing
  (:Pressed
    (Variables|Default|SetAttackSelect (+ (Variables|Default|GetAttackSelect) 1))
    (if (== (Variables|Default|GetAttackSelect) 4)
      (Variables|Default|SetAttackSelect 0))
    (switch int (Variables|Default|GetAttackSelect)
      (:0
        (Variables|Default|SetPowerSelect "NewEnumerator0"))
      (:1
        (Variables|Default|SetPowerSelect "NewEnumerator1"))
      (:2
        (Variables|Default|SetPowerSelect "NewEnumerator2"))
      (:3
        (Variables|Default|SetPowerSelect "NewEnumerator3")))
    (Development|PrintString (Utilities|String|EnumtoString (Variables|Default|GetPowerSelect)))))

(fn ConstructionScript)

(fn CloseGate
  (CallFunction|CloseIceShard)
  (CallFunction|CloseLightningOrb)
  (CallFunction|CloseArcaneBlade))

(fn CloseGateAlt
  (Utilities|FlowControl|Sequence))

(fn LeftRightTilt
  (params (Axis%20Value :type Float%20%28single-precision%29))
  (Variables|Default|SetBanking (Math|Float|Clamp(Float) (+ (Variables|Default|GetBanking) (* Axis%20Value 2.0)) -3e+01 3e+01)))

(fn AutofireFunct
  (CallFunction|Autofireball)
  (CallFunction|IceShardAuto)
  (CallFunction|LightningOrbAuto)
  (CallFunction|FlameBreathTick)
  (CallFunction|ArcaneBladeAuto))