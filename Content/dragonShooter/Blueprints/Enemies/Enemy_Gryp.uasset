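; Gryphon enemy child Blueprint that sets its health and adds a falling death sequence to its parent class.
; The parent's death-sequence dispatcher, re-bound every Tick, enables physics on the collision sphere so the body drops.
; Tick then plays death and fall animations while sphere-tracing for a surface.
; On a hit, it stops physics, plays impact and dead animations, then destroys the actor after a delay.
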(event Custom|Death
  (Variables|Default|Setphysicssim true)
  (Physics|SetSimulatePhysics (Variables|Default|GetSphereCollision) (Variables|Default|Getphysicssim)))

(event EventBeginPlay
  (|CallParentFunction)
  (Variables|Default|SetHealth (Variables|Default|GetGryphonHealth)))

(event Collision|EventActorBeginOverlap
  (params (OtherActor :type Actor%20Object%20Reference))
  (|CallParentFunction OtherActor) ; This node is disabled and will not be called.\nDrag off pins to build functionality.
)

(event EventTick
  (params (DeltaSeconds :type Float%20%28single-precision%29))
  (bind _sphere (Variables|Default|GetSphere))
  (bind _skeletalmesh (Variables|Default|GetSkeletalMesh))
  (bind _returnvalue (Transformation|GetWorldLocation _sphere))
  (|CallParentFunction DeltaSeconds)
  (EventDispatchers|BindEventtoStartDeathSequence (delegate Custom|Death))
  (if (Variables|Default|Getphysicssim)
    (Utilities|FlowControl|Sequence
      (:then_0
        (Utilities|FlowControl|DoOnce false
          (:Completed
            (Components|Animation|PlayAnimation _skeletalmesh "/Game/QuadrapedCreatures/Griffon/Animations/Death.Death" false)
            (Utilities|FlowControl|Delay 1.0)
            (Components|Animation|PlayAnimation _skeletalmesh "/Game/QuadrapedCreatures/Griffon/Animations/DeathFall.DeathFall" (Variables|Default|GetLoop)))))
      (:then_1
        (bind _returnvalue_2 (Collision|SphereTraceForObjects _returnvalue (+ _returnvalue (* (Transformation|GetActorUpVector) 1.0)) (Components|Sphere|GetScaledSphereRadius _sphere) (Variables|Default|GetTrace) false 0 "None" true "(R=1.000000,G=0.000000,B=0.000000,A=1.000000)" "(R=0.000000,G=1.000000,B=0.000000,A=1.000000)" 0.0))
        (if _returnvalue_2
          (Utilities|FlowControl|DoOnce false
            (:Completed
              (Physics|SetSimulatePhysics (Variables|Default|GetSphereCollision) false)
              (Components|Animation|PlayAnimation (Variables|Default|GetSkeletalMesh) "/Game/QuadrapedCreatures/Griffon/Animations/ANIM_Griffon_HitTheGround.ANIM_Griffon_HitTheGround" false)
              (Variables|Default|SetLoop false)
              (Utilities|FlowControl|Delay 0.667)
              (Components|Animation|PlayAnimation (Variables|Default|GetSkeletalMesh) "/Game/QuadrapedCreatures/Griffon/Animations/SK_Griffon_Dead.SK_Griffon_Dead" true)
              (Utilities|FlowControl|Delay 3.0)
              (Actor|DestroyActor))))))))

(fn ConstructionScript
  (|CallParentFunction))