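; Harpy enemy Blueprint that sets its health on BeginPlay and plays a physics-driven falling death.
; Tick rebinds Death to the StartDeathSequence dispatcher every frame; Death enables physics simulation on the collision sphere.
; While falling, Tick plays hit and fall animations once and sphere-traces for ground contact.
; On contact it stops physics, plays impact and dead animations, then destroys the actor after a delay.
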(event Custom|Death
  (Variables|Default|Setphysicssim true)
  (Physics|SetSimulatePhysics (Variables|Default|GetSphereCollision) (Variables|Default|Getphysicssim)))

(event EventBeginPlay
  (|CallParentFunction)
  (Variables|Default|SetHealth (Variables|Default|GetHarpyHealth)))

(event Collision|EventActorBeginOverlap
  (params (OtherActor :type Actor%20Object%20Reference))
  (|CallParentFunction OtherActor) ; This node is disabled and will not be called.\nDrag off pins to build functionality.
)

(event EventTick
  (params (DeltaSeconds :type Float%20%28single-precision%29))
  (bind _sphere (Variables|Default|GetSphere))
  (bind _skeletalmesh (Variables|Default|GetSkeletalMesh))
  (bind _returnvalue (Transformation|GetWorldLocation _sphere))
  (|CallParentFunction DeltaSeconds)
  (EventDispatchers|BindEventtoStartDeathSequence (delegate Custom|Death))
  (if (Variables|Default|Getphysicssim)
    (Utilities|FlowControl|Sequence
      (:then_0
        (Utilities|FlowControl|DoOnce false
          (:Completed
            (Components|Animation|PlayAnimation _skeletalmesh "/Game/QuadrapedCreatures/Harpy/Animations/ANIM_HARPY_getHitToFall.ANIM_HARPY_getHitToFall" false)
            (Utilities|FlowControl|Delay 1.167)
            (Components|Animation|PlayAnimation _skeletalmesh "/Game/QuadrapedCreatures/Harpy/Animations/ANIM_HARPY_falling.ANIM_HARPY_falling" (Variables|Default|GetLoop)))))
      (:then_1
        (bind _returnvalue_2 (Collision|SphereTraceForObjects _returnvalue (+ _returnvalue (* (Transformation|GetActorUpVector) 1.0)) (Components|Sphere|GetScaledSphereRadius _sphere) (Variables|Default|GetTrace) false 0 "ForDuration" true "(R=1.000000,G=0.000000,B=0.000000,A=1.000000)" "(R=0.000000,G=1.000000,B=0.000000,A=1.000000)" 0.0))
        (if _returnvalue_2
          (Utilities|FlowControl|DoOnce false
            (:Completed
              (Physics|SetSimulatePhysics (Variables|Default|GetSphereCollision) false)
              (Components|Animation|PlayAnimation (Variables|Default|GetSkeletalMesh) "/Game/QuadrapedCreatures/Harpy/Animations/ANIM_HARPY_deathHitTheGround.ANIM_HARPY_deathHitTheGround" false)
              (Variables|Default|SetLoop false)
              (Utilities|FlowControl|Delay 0.667)
              (Components|Animation|PlayAnimation (Variables|Default|GetSkeletalMesh) "/Game/QuadrapedCreatures/Harpy/Animations/HARPY_Dead.HARPY_Dead" true)
              (Utilities|FlowControl|Delay 3.0)
              (Actor|DestroyActor))))))))

(fn ConstructionScript
  (|CallParentFunction))