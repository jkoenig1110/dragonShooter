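; Base enemy for the dragon shooter that flies along a spline, takes damage and can drop an ability pickup.
; ActivateEnemy plays a timeline scaled by spline length and EnemySpeed, moving the collision sphere at constant velocity.
; Any and radial damage reduce Health, triggering a one-time death sequence that stops movement and deactivates the spline.
; A drop roll made at BeginPlay decides whether death spawns a randomly typed Ability_Pickup.
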(event Custom|ActivateEnemy
  (Components|Timeline|SetPlayRate (Variables|Default|GetEnemyMovementTimeline) (/ 1.0 (/ (Spline|GetSplineLength (Variables|Default|GetSpline)) (Variables|Default|GetEnemySpeed))))
  (bind _movementsplineloc (Timeline|EnemyMovementTimeline PlayFromStart)
    (:Update
      (Transformation|SetWorldLocation (Variables|Default|GetSphereCollision) (Spline|GetLocationatTime (Variables|Default|GetSpline) _movementsplineloc "World" true) false false))))

(event Custom|Dead
  (bind _movementsplineloc (Timeline|EnemyMovementTimeline Stop)
    (:Update
      (Transformation|SetWorldLocation (Variables|Default|GetSphereCollision) (Spline|GetLocationatTime (Variables|Default|GetSpline) _movementsplineloc "World" true) false false))))

(event EventBeginPlay
  (Utilities|FlowControl|Sequence
    (:then_0
      (bind _outactors (Actor|GetAllActorsOfClass "/Game/dragonShooter/Blueprints/PlayField.Playfield_C"))
      (Variables|Default|SetPlayfieldRef (Utilities|Array|Get(acopy) _outactors)))
    (:then_1
      (Variables|Default|SetDropCHance (Math|Random|RandomIntegerinRange 1 (Variables|Default|GetMaxChance))))))

(event Collision|EventActorBeginOverlap
  (params (OtherActor :type Actor%20Object%20Reference)))

(event EventTick
  (params (DeltaSeconds :type Float%20%28single-precision%29)))

(event Game|Damage|EventRadialDamage
  (params (DamageReceived :type Float%20%28single-precision%29) (DamageType :type Damage%20Type%20Object%20Reference) (Origin :type Vector :default "0, 0, 0") (HitInfo :type Hit%20Result%20Structure%20%28by%20ref%29) (InstigatedBy :type Controller%20Object%20Reference) (DamageCauser :type Actor%20Object%20Reference))
  (Variables|Default|SetHealth (- (Variables|Default|GetHealth) DamageReceived))
  (if (<= (Variables|Default|GetHealth) 0.0)
    (Utilities|FlowControl|DoOnce false
      (:Completed
        (Utilities|FlowControl|Sequence
          (:then_0
            (Default|CallStartDeathSequence)
            (Transformation|DetachFromActor (Variables|Default|GetPlayfieldRef) "KeepWorld" "KeepWorld" "KeepWorld")
            (CallFunction|Dead)
            (Components|Activation|Deactivate (Variables|Default|GetSpline)))
          (:then_1
            (if (== (Variables|Default|GetDropCHance) 1)
              (Game|SpawnActorfromClass "/Game/dragonShooter/Projectiles/Ability_Pickup.Ability_Pickup_C" (Transformation|GetWorldTransform (Variables|Default|GetSphereCollision)) "Undefined" 0 (Utilities|Select :Index (Math|Random|RandomIntegerinRange 0 3) :Option%200 "NewEnumerator0" :Option%201 "NewEnumerator1" :Option%202 "NewEnumerator2" :Option%203 "NewEnumerator3") 0))))))))

(event Game|Damage|EventAnyDamage
  (params (Damage :type Float%20%28single-precision%29) (DamageType :type Damage%20Type%20Object%20Reference) (InstigatedBy :type Controller%20Object%20Reference) (DamageCauser :type Actor%20Object%20Reference))
  (Variables|Default|SetHealth (- (Variables|Default|GetHealth) Damage))
  (if (<= (Variables|Default|GetHealth) 0.0)
    (Utilities|FlowControl|DoOnce false
      (:Completed
        (Utilities|FlowControl|Sequence
          (:then_0
            (Default|CallStartDeathSequence)
            (Transformation|DetachFromActor (Variables|Default|GetPlayfieldRef) "KeepWorld" "KeepWorld" "KeepWorld")
            (CallFunction|Dead)
            (Components|Activation|Deactivate (Variables|Default|GetSpline)))
          (:then_1
            (if (== (Variables|Default|GetDropCHance) 1)
              (Game|SpawnActorfromClass "/Game/dragonShooter/Projectiles/Ability_Pickup.Ability_Pickup_C" (Transformation|GetWorldTransform (Variables|Default|GetSphereCollision)) "Undefined" 0 (Utilities|Select :Index (Math|Random|RandomIntegerinRange 0 3) :Option%200 "NewEnumerator0" :Option%201 "NewEnumerator1" :Option%202 "NewEnumerator2" :Option%203 "NewEnumerator3") 0))))))))

(fn ConstructionScript)